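; BP_MP_PC is a multiplayer player controller with logic to register its BP_MP_Pawn with Main_HUD.
; Two custom events cast the controlled pawn and HUD, then store the pawn in the HUD's C1 or C2 slot.
; A delayed Player1/Player2 tag check that would choose between them is disconnected, and BeginPlay is empty.
; Get Character Info is a stub returning zero speed and false for every movement and state flag.
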(event Custom|CustomEvent_1
  (bind _asbp_mp_pawn_c (Utilities|Casting|CastToBP_MP_Pawn (Pawn|GetControlledPawn)))
  (bind _asmain_hud_c (Utilities|Casting|CastToMain_HUD (HUD|GetHUD)))
  (Variables|/Game/HUD/Main_HUD.Main_HUD_C|SetC1 _asmain_hud_c _asbp_mp_pawn_c))

(event Custom|CustomEvent_3
  (bind _asbp_mp_pawn_c (Utilities|Casting|CastToBP_MP_Pawn (Pawn|GetControlledPawn)))
  (bind _asmain_hud_c (Utilities|Casting|CastToMain_HUD (HUD|GetHUD)))
  (Variables|/Game/HUD/Main_HUD.Main_HUD_C|SetC2 _asmain_hud_c _asbp_mp_pawn_c))

(event EventBeginPlay)

(fn ConstructionScript)

(fn GetCharacterInfo
  (return 0.0 false false false false false false false false false))