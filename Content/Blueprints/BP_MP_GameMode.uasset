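; Two-player game mode that assigns player starts and drives a camera offset on each BP_MP_Pawn based on the distance between the players.
; PostLogin stores each controller and pawn, then repeats SetCameraOffSet on a short Delay loop once Character2 exists.
; Offsets use half-separations and 45-degree tangent depth, signed by Y order, before calling MovimientoCamera on both pawns.
; ChoosePlayerStart uses the "Taken" tag to mark used starts.
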(event EventPostLogin
  (params (NewPlayer :type Player%20Controller%20Object%20Reference))
  (CallFunction|StorePlayer NewPlayer)
  (Development|PrintString "game")
  (if (not (== (Variables|Default|GetCharacter2) 0))
    (CallFunction|SetCameraOffSet :!label _label)
    (Utilities|FlowControl|Delay 0.15)
    (goto _label)))

(fn ConstructionScript)

(fn CalculateCameraPosition
  (bind _distance (CallFunction|DistanceBetweenCharactersHorizontal))
  (bind _distance_2 (CallFunction|DistanceBetweenCharactersVertical))
  (bind _distance_3 (CallFunction|CalculateDepth))
  (LocalVariables|SetCalculatedOffSet (Math|Vector|MakeVector _distance_3 _distance _distance_2))
  (return (LocalVariables|GetCalculatedOffSet)))

(fn DistanceBetweenCharactersHorizontal
  (bind _returnvalue (Transformation|GetHorizontalDistanceTo (Variables|Default|GetCharacter1) (Variables|Default|GetCharacter2)))
  (return (/ _returnvalue 2.0)))

(fn DistanceBetweenCharactersVertical
  (bind _returnvalue (Class|Actor|GetVerticalDistanceto (Variables|Default|GetCharacter1) (Variables|Default|GetCharacter2)))
  (return (/ _returnvalue 2.0)))

(fn CalculateDepth
  (bind _returnvalue (Transformation|GetDistanceTo (Variables|Default|GetCharacter1) (Variables|Default|GetCharacter2)))
  (return (/ (/ _returnvalue 2.0) (Math|Trig|Tan(Degrees) 45.0))))

(fn SetCameraOffSet
  (bind _character2 (Variables|Default|GetCharacter2))
  (bind _character1 (Variables|Default|GetCharacter1))
  (bind _character2_2 (Variables|Default|GetCharacter2))
  (bind _character1_2 (Variables|Default|GetCharacter1))
  ;[1 1 1] Almacena el ultimo calculo de la posicion de la camara
  (Variables|/Game/Blueprints/BP_MP_Pawn.BP_MP_Pawn_C|SetOldCameraLocationOffset _character1_2 (Variables|/Game/Blueprints/BP_MP_Pawn.BP_MP_Pawn_C|GetCameraLocationOffset _character1_2))
  (Variables|/Game/Blueprints/BP_MP_Pawn.BP_MP_Pawn_C|SetOldCameraLocationOffset _character2 (Variables|/Game/Blueprints/BP_MP_Pawn.BP_MP_Pawn_C|GetCameraLocationOffset _character2))
  ;[1 1 1] Calcula la siguiente posicion de la camara
  (bind _location (CallFunction|CalculateCameraPosition))
  (LocalVariables|SetTemporaryLocation _location)
  ;[1 1 1] If posicion
  (if (> (.Y (Math|Vector|BreakVector (Transformation|GetActorLocation (Variables|Default|GetCharacter1)))) (.Y (Math|Vector|BreakVector (Transformation|GetActorLocation (Variables|Default|GetCharacter2)))))
    ;[1 1 1] Almacena la nueva posicion a la que debe dirigirse la camara si el player 1 esta a la derecha de la pantalla
    (Variables|/Game/Blueprints/BP_MP_Pawn.BP_MP_Pawn_C|SetCameraLocationOffset (Variables|Default|GetCharacter2) (Math|Vector|MakeVector (* (.X (Math|Vector|BreakVector (LocalVariables|GetTemporaryLocation))) -1.0) (* (.Y (Math|Vector|BreakVector (LocalVariables|GetTemporaryLocation))) -1.0) (* (.Z (Math|Vector|BreakVector (LocalVariables|GetTemporaryLocation))) -1.0)))
    (Variables|/Game/Blueprints/BP_MP_Pawn.BP_MP_Pawn_C|SetCameraLocationOffset (Variables|Default|GetCharacter1) (Math|Vector|MakeVector (* (.X (Math|Vector|BreakVector (LocalVariables|GetTemporaryLocation))) -1.0) (* (.Y (Math|Vector|BreakVector (LocalVariables|GetTemporaryLocation))) 1.0) (* (.Z (Math|Vector|BreakVector (LocalVariables|GetTemporaryLocation))) 1.0)))
    ;[1 1 1] Evento para mover la camara
    (Default|MovimientoCamera _character2_2)
    (Default|MovimientoCamera _character1)
    (else
      ;[1 1 1] Almacena la nueva posicion a la que debe dirigirse la camara si el player 1 esta a la izquierda de la pantalla
      (Variables|/Game/Blueprints/BP_MP_Pawn.BP_MP_Pawn_C|SetCameraLocationOffset (Variables|Default|GetCharacter1) (Math|Vector|MakeVector (* (.X (Math|Vector|BreakVector (LocalVariables|GetTemporaryLocation))) -1.0) (* (.Y (Math|Vector|BreakVector (LocalVariables|GetTemporaryLocation))) -1.0) (* (.Z (Math|Vector|BreakVector (LocalVariables|GetTemporaryLocation))) 1.0)))
      (Variables|/Game/Blueprints/BP_MP_Pawn.BP_MP_Pawn_C|SetCameraLocationOffset (Variables|Default|GetCharacter2) (Math|Vector|MakeVector (* (.X (Math|Vector|BreakVector (LocalVariables|GetTemporaryLocation))) -1.0) (* (.Y (Math|Vector|BreakVector (LocalVariables|GetTemporaryLocation))) 1.0) (* (.Z (Math|Vector|BreakVector (LocalVariables|GetTemporaryLocation))) -1.0)))
      (Default|MovimientoCamera _character1)
      (Default|MovimientoCamera _character2_2))))

(fn ChoosePlayerStart
  (bind _outactors (Actor|GetAllActorsOfClass "/Script/Engine.PlayerStart"))
  (bind _array_element (Utilities|Array|ForEachLoopwithBreak _outactors :!label _label)
    (:LoopBody
      (bind _asplayerstart (Utilities|Casting|CastToPlayerStart _array_element))
      (if (Utilities|Name|NotEqual(Name) (Variables|/Script/Engine.PlayerStart|GetPlayerStartTag _asplayerstart) "Taken")
        (Utilities|FlowControl|Sequence
          (:then_0
            (goto _label Break))
          (:then_1
            (Variables|/Script/Engine.PlayerStart|SetPlayerStartTag _asplayerstart "Taken"))
          (:then_2
            (return _asplayerstart)))))))

(fn StorePlayer
  (params (PlayerControllerInput :type Player%20Controller%20Object%20Reference))
  (if (!= (Variables|Default|GetPlayerController1) 0)
    (if (not (!= (Variables|Default|GetPlayerController2) 0))
      (Variables|Default|SetPlayerController2 PlayerControllerInput)
      (bind _asbp_mp_pawn_c (Utilities|Casting|CastToBP_MP_Pawn (Pawn|GetControlledPawn (Variables|Default|GetPlayerController2))))
      (Variables|Default|SetCharacter2 _asbp_mp_pawn_c))
    (else
      (Variables|Default|SetPlayerController1 PlayerControllerInput)
      (bind _asbp_mp_pawn_c_2 (Utilities|Casting|CastToBP_MP_Pawn (Pawn|GetControlledPawn (Variables|Default|GetPlayerController1))))
      (Variables|Default|SetCharacter1 _asbp_mp_pawn_c_2))))